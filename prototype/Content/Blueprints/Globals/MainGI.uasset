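; MainGI appears to be the game instance that handles multiplayer menus and sessions.
; It lazily creates, caches and shows the SearchGame and HostGame widgets.
; LaunchLobby stores the server name, creates a 20-connection online session and opens Level1 as a listen server, ignoring its UsingSteam input.
; JoinGame joins a supplied search result and only prints success or failure, with no explicit travel.
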(event Custom|ShowSearchGames
  (Utilities|IsValid (Variables|Default|GetSearchGames)
    (:Is%20Valid
      _)
    (:Is%20Not%20Valid
      (bind _returnvalue (UserInterface|CreateWidget "/Game/Blueprints/Menus/SearchGame.SearchGame_C" (Game|GetPlayerController 0)))
      (bind _output_get (Variables|Default|SetSearchGames _returnvalue))))
  (UserInterface|Viewport|AddtoViewport _output_get 0))

(event Custom|JoinGame
  (params (SessionToJoin :type Blueprint%20Session%20Result%20Structure))
  (|JoinSession (Game|GetPlayerController 0) SessionToJoin
    (:OnSuccess
      (Development|PrintString "Joined"))
    (:OnFailure
      (Development|PrintString "Failed to join"))))

(event Custom|LaunchLobby
  (params (ServerName :type Text) (UsingSteam :type Boolean))
  (Variables|Default|SetServerName ServerName)
  (|Session (Game|GetPlayerController 0) 20 false
    (:OnSuccess
      (Game|OpenLevel(byName) "Level1" true "listen"))
    (:OnFailure
      (Development|PrintString "Failed"))))

(event Custom|HostGameMenu
  (Utilities|IsValid (Variables|Default|GetHostGame)
    (:Is%20Valid
      _)
    (:Is%20Not%20Valid
      (bind _returnvalue (UserInterface|CreateWidget "/Game/Blueprints/Menus/HostGame.HostGame_C" (Game|GetPlayerController 0)))
      (bind _output_get (Variables|Default|SetHostGame _returnvalue))))
  (UserInterface|Viewport|AddtoViewport _output_get 0))